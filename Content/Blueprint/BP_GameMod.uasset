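; Game mode that drives a rock-spawning game with escalating difficulty and relays start, end and restart events to BP_GameState.
; BeginPlay caches the game state and starts the game.
; Each Process call checks the supplied time and, on every multiple of five, spawns a BP_Rock at a random XY within fixed bounds at constant height, then tells the game state to increase difficulty.
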(event `self.ReceiveBeginPlay`
  (bind _asbp_game_state (cast `/Game/Blueprint/BP_GameState` (`GameplayStatics.GetGameState`)))
  (bind _output_get (set `self.As BP Game State` _asbp_game_state))
  (`/Game/Blueprint/BP_GameState.StartGameEvent` _output_get))

(event `Process`
  (params (CurrentTime :type Integer))
  (if (== (mod CurrentTime 5) 0)
    (`self.SpawnRock`)
    (`/Game/Blueprint/BP_GameState.IncreaseDifficulty` (`self.As BP Game State`))))

(event `End`
  (`/Game/Blueprint/BP_GameState.EndGameEvent` (`self.As BP Game State`)))

(event `Restart`
  (`/Game/Blueprint/BP_GameState.RestartGameEvent` (`self.As BP Game State`)))

(fn `SpawnRock`
  (`|SpawnActorFromClass` "/Game/Blueprint/BP_Rock.BP_Rock_C" (`KismetMathLibrary.MakeTransform` (`KismetMathLibrary.MakeVector` (`KismetMathLibrary.RandomFloatInRange` -1700.0 900.0) (`KismetMathLibrary.RandomFloatInRange` -1300.0 1300.0) 250.0)) "AdjustIfPossibleButAlwaysSpawn" "OverrideRootScale" null null))

(fn `UserConstructionScript`)