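; BP_GameState tracks the match clock, difficulty and game-over flag, and drives the start, end and restart flow.
; A looping one-second timer counts time played, adds the current difficulty to every player's score and passes the elapsed time to BP_GameMod for processing.
; Ending clears the timer and submits each player's score to BP_GameInstance as a high-score candidate, while restarting reopens the current level.
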(event `self.ReceiveBeginPlay`)

(event `StartGameEvent`
  (bind _returnvalue (`KismetSystemLibrary.K2_SetTimerDelegate` (delegate `MainTImerEvent`) 1.0 true))
  (set `self.Timer` _returnvalue)
  (set `self.IsGameEnded` false))

(event `MainTImerEvent`
  (`/Engine/EditorBlueprintResources/StandardMacros.IncrementInt` (`self.TimePlayed`)
    (:`  `
      (for _array_element (`self.PlayerArray`)
        (bind _asbp_player_state (cast `/Game/Blueprint/BP_PlayerState` _array_element))
        (`/Game/Blueprint/BP_PlayerState.AddPlayerScore` _asbp_player_state (`self.Difficult`)))
      (bind _asbp_game_mod (cast `/Game/Blueprint/BP_GameMod` (`GameplayStatics.GetGameMode`)))
      (`/Game/Blueprint/BP_GameMod.Process` _asbp_game_mod (`self.TimePlayed`)))))

(event `EndGameEvent`
  (`KismetSystemLibrary.K2_ClearAndInvalidateTimerHandle` (`self.Timer`))
  (set `self.IsGameEnded` true)
  (bind _asbp_game_instance (cast `/Game/Blueprint/BP_GameInstance` (`GameplayStatics.GetGameInstance`)))
  (for _array_element (`self.PlayerArray`)
    (bind _asbp_player_state (cast `/Game/Blueprint/BP_PlayerState` _array_element))
    (`/Game/Blueprint/BP_GameInstance.UpdateHighestScore` _asbp_game_instance (`/Game/Blueprint/BP_PlayerState.GetPlayerScore` _asbp_player_state))))

(event `RestartGameEvent`
  (bind _returnvalue (`GameplayStatics.GetCurrentLevelName` true))
  (`GameplayStatics.OpenLevel` (`KismetStringLibrary.Conv_StringToName` _returnvalue)))

(fn `GetDifficulty`
  (returns (Difficult :type Integer))
  (return (`self.Difficult`)))

(fn `GetGameEnded`
  (returns (IsGameEnded :type Boolean))
  (return (`self.IsGameEnded`)))

(fn `GetTimePlayed`
  (returns (TimePlayed :type Integer))
  (return (`self.TimePlayed`)))

(fn `IncreaseDifficulty`
  (`/Engine/EditorBlueprintResources/StandardMacros.IncrementInt` (`self.Difficult`)))

(fn `UserConstructionScript`)