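; BP_MaterialCOntroller is a trigger actor that keeps randomly recoloring BP_CubeTarget actors while something overlaps its Box.
; Begin overlap starts a looping one-second timer whose event gets every BP_CubeTarget and sets its Cube material to a random array pick.
; End overlap clears the timer through the stored handle.
; A switch mapping a Color value to colored material instances is left unconnected and never runs.
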(event `self.Box.OnComponentBeginOverlap`
  (params (OverlappedComponent :type "PrimitiveComponent Object Reference") (OtherActor :type "Actor Object Reference") (OtherComp :type "PrimitiveComponent Object Reference") (OtherBodyIndex :type Integer) (bFromSweep :type Boolean) (SweepResult :type "HitResult Structure (by ref)"))
  (bind _returnvalue (`KismetSystemLibrary.K2_SetTimerDelegate` (delegate `EventColor`) 1.0 true))
  (set `self.NewVar_2` _returnvalue))

(event `EventColor`
  (bind _outactors (`GameplayStatics.GetAllActorsOfClass` "/Game/10_5/BP_CubeTarget.BP_CubeTarget_C"))
  (for _array_element _outactors
    (`PrimitiveComponent.SetMaterial` (`/Game/10_5/BP_CubeTarget.Cube` _array_element) 0 (`KismetArrayLibrary.Array_Random` (`self.Cube`)))))

(event `self.Box.OnComponentEndOverlap`
  (params (OverlappedComponent :type "PrimitiveComponent Object Reference") (OtherActor :type "Actor Object Reference") (OtherComp :type "PrimitiveComponent Object Reference") (OtherBodyIndex :type Integer))
  (`KismetSystemLibrary.K2_ClearAndInvalidateTimerHandle` (`self.NewVar_2`)))

(fn `UserConstructionScript`)