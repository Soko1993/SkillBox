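; BP_Actor is an overlap-triggered pickup that grants the third-person character health, armor or energy.
; On actor overlap it casts the other actor to ThirdPersonCharacter, then switches on its Type to call the matching AddHealth, AddArmor or AddEnergy function.
; The actor stays in the world after granting the bonus.
; The remaining array, set, map, level-load and quit nodes are disconnected and never run.
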(event `self.ReceiveActorBeginOverlap`
  (params (OtherActor :type "Actor Object Reference"))
  (bind _asthird_person_character (cast `/Game/ThirdPersonBP/Blueprints/ThirdPersonCharacter` OtherActor))
  (switch `/Game/9_1/EBonusTypes` (`self.Type`)
    (:`NewEnumerator0`
      (`/Game/ThirdPersonBP/Blueprints/ThirdPersonCharacter.AddHealth` _asthird_person_character))
    (:`NewEnumerator1`
      (`/Game/ThirdPersonBP/Blueprints/ThirdPersonCharacter.AddArmor` _asthird_person_character))
    (:`NewEnumerator2`
      (`/Game/ThirdPersonBP/Blueprints/ThirdPersonCharacter.AddEnergy` _asthird_person_character))))

(fn `UserConstructionScript`)